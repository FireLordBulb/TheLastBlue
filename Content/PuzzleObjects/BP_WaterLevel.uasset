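; BP_WaterLevel is a puzzle object that animates a water plane to the height of a new water level.
; Level changes arrive through a WaterLevel event binding or as relative amounts, and a Timeline lerps the plane's Z to the height mapped to that enum value.
; A draining sound plays until the Timeline finishes, when a dispatcher fires.
; At the WaterGone level the actor hides and disables the plane's collision.
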(event Custom|ChangeWaterLevelBy
  (params (Amount :type Byte))
  (CallFunction|SetNewWaterLevel (Utilities|Enum|ByteToEnumEWaterLevel (+ Amount (Variables|Default|GetCurrentWaterLevel)))))

(event Custom|SetNewWaterLevel
  (params (CurrentWaterLevel :type EWaterLevel%20Enum :default "MaxWater"))
  (Variables|Default|SetTempPosition (Variables|/Script/Engine.SceneComponent|GetRelativeLocation (Variables|Default|GetWaterPlane)))
  (bind _returnvalue (Audio|SpawnSound2D "/Game/Audio/SFX/OneShots/MetaSoundSources/MSS_DrainingWater.MSS_DrainingWater" 1.0 1.0 0.0 0))
  (Variables|Default|SetSFXDrainingWater _returnvalue)
  (bind _time (Timeline|Timeline PlayFromStart)
    (:Update
      (Transformation|SetRelativeLocation (Variables|Default|GetWaterPlane) (Math|Vector|MakeVector (.x (Variables|Default|GetTempPosition)) (.y (Variables|Default|GetTempPosition)) (Math|Float|Lerp (.z (Variables|Default|GetTempPosition)) (.Value (Utilities|Map|Find (Variables|Default|GetEWater%20Lowering) CurrentWaterLevel)) _time)) false false))
    (:Finished
      (Class|AudioParameterControllerInterface|SetTriggerParameter(Message) (Variables|Default|GetSFXDrainingWater) "FinishPlaying")
      (Default|CallWaterLevelLoweredDispatcher)
      (Variables|Default|SetCurrentWaterLevel CurrentWaterLevel)
      (if (Utilities|Enum|Equal(Enum) "WaterGone" CurrentWaterLevel)
        (Rendering|SetActorHiddenInGame true)
        (Collision|SetCollisionEnabled (Variables|Default|GetWaterPlane) "NoCollision")))))

(event EventBeginPlay
  (EventDispatchers|BindEventtoRaise (Variables|Default|GetWaterLevel) (delegate Custom|SetNewWaterLevel)))

(event Collision|EventActorBeginOverlap
  (params (OtherActor :type Actor%20Object%20Reference)))

(event EventTick
  (params (DeltaSeconds :type Float%20%28single-precision%29)))

(fn ConstructionScript)