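; BP_Laser is a powerable puzzle laser whose beam knocks back characters on hit.
; While powered, Tick traces along the beam's up vector, ignoring the player pawn, and scales BeamParent to end at the first blocker or maximum length.
; Power-off collapses the beam to zero length.
; Hit zeroes the character's velocity, then applies an impulse horizontally away from the hit point with an upward component.
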(event EventBeginPlay
  (bind _beamdiameterscale (Variables|Default|GetBeamDiameterScale))
  (Transformation|SetRelativeScale3D (Variables|Default|GetBeam) (Math|Vector|MakeVector _beamdiameterscale _beamdiameterscale 1.0))
  (if (Variables|Default|GetIsPowered)
    _
    (else
      (Utilities|SetBeamLength 0.0)))
  (if (>= (Variables|Default|GetBeamDiameterScale) 0.04)
    (Rendering|Material|SetScalarParameterValueonMaterials (Variables|Default|GetBeam) "Brightness" 0.3)))

(event EventTick
  (params (DeltaSeconds :type Float%20%28single-precision%29))
  (bind _beamparent (Variables|Default|GetBeamParent))
  (bind _returnvalue (Transformation|GetWorldLocation _beamparent))
  (if (Variables|Default|GetIsPowered)
    (bind _outhit (Collision|LineTraceByChannel _returnvalue (+ _returnvalue (* (Math|Vector|GetUpVector (Transformation|GetWorldRotation _beamparent)) (Variables|Default|GetMaxBeamLength))) "TraceTypeQuery1" false (Utilities|Array|MakeArray (Game|Player|GetPlayerPawn 0)) "None"))
    (if (.bblockinghit _outhit)
      (Utilities|SetBeamLength (.distance _outhit))
      (else
        (Utilities|SetBeamLength (Variables|Default|GetMaxBeamLength))))))

(event EventOnPoweron
  (Variables|Default|SetIsPowered true))

(event EventOnPowerOff
  (Variables|Default|SetIsPowered false)
  (Utilities|SetBeamLength 0.0))

(event Collision|EventHit
  (params (MyComp :type Primitive%20Component%20Object%20Reference) (Other :type Actor%20Object%20Reference) (OtherComp :type Primitive%20Component%20Object%20Reference) (bSelfMoved :type Boolean) (HitLocation :type Vector :default "0, 0, 0") (HitNormal :type Vector :default "0, 0, 0") (NormalImpulse :type Vector :default "0, 0, 0") (Hit :type Hit%20Result%20Structure%20%28by%20ref%29))
  (bind _returnvalue (Transformation|GetActorLocation Other))
  (bind _returnvalue_2 (- _returnvalue HitLocation))
  (bind _returnvalue_3 (Math|Vector2D|MakeVector2D (.x _returnvalue_2) (.y _returnvalue_2)))
  (bind _returnvalue_4 (Math|Vector2D|Normalize2D _returnvalue_3))
  (bind _ascharacter (Utilities|Casting|CastToCharacter Other))
  (Variables|/Script/Engine.MovementComponent|SetVelocity (Variables|/Script/Engine.Character|GetCharacterMovement _ascharacter) "0, 0, 0")
  (Physics|AddImpulse (Variables|/Script/Engine.Character|GetCharacterMovement _ascharacter) (* (Math|Vector|MakeVector (.x _returnvalue_4) (.y _returnvalue_4) (Variables|Default|GetUpKnockbackComponent)) (Variables|Default|GetKnockbackImpulse)) false))

(fn ConstructionScript)

(fn GetGlyphProvider
  (return 0))