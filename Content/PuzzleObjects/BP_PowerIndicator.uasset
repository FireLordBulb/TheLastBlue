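; Puzzle power indicator that shows its powered state through the emissive intensity of its static mesh material.
; Power on and off events increment or decrement a puzzle counter, play timelines that fade the glow, then set IsPowered when finished.
; While powered, Tick drives a pulse timeline between on and pulse intensities.
; LightUp and LightDown fade the glow without changing power state or counter; BeginPlay initializes emissive intensity through TurnOnOff.
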(event Custom|Event%20Light%20Up
  (bind _timetoon (Timeline|Timeline Play)
    (:Update
      (Rendering|Material|SetScalarParameterValueonMaterials (Variables|Default|GetStaticMesh) "emissive intensity" (Math|Float|Lerp (Variables|Default|GetTurnedOffIntensity) (Variables|Default|GetTurnedOnIntensity) _timetoon)))))

(event Custom|Event%20Light%20Down
  (bind _timetoon (Timeline|Timeline_0 Play)
    (:Update
      (Rendering|Material|SetScalarParameterValueonMaterials (Variables|Default|GetStaticMesh) "emissive intensity" (Math|Float|Lerp (Variables|Default|GetTurnedOnIntensity) (Variables|Default|GetTurnedOffIntensity) _timetoon)))))

(event EventBeginPlay
  (CallFunction|TurnonOff))

(event Collision|EventActorBeginOverlap
  (params (OtherActor :type Actor%20Object%20Reference)))

(event EventTick
  (params (DeltaSeconds :type Float%20%28single-precision%29))
  (if (Variables|Default|GetIsPowered)
    (bind _newtrack_0 (Timeline|PulsateTimeline Play)
      (:Update
        (Rendering|Material|SetScalarParameterValueonMaterials (Variables|Default|GetStaticMesh) "emissive intensity" (Math|Float|Lerp (Variables|Default|GetTurnedOnIntensity) (Variables|Default|GetPulseIntensity) _newtrack_0))))
    (else
      (Timeline|PulsateTimeline Stop))))

(event EventOnPoweron
  (Default|CallIncrementPuzzleCounter)
  (bind _timetoon (Timeline|TimeToOn PlayFromStart)
    (:Update
      (Rendering|Material|SetScalarParameterValueonMaterials (Variables|Default|GetStaticMesh) "emissive intensity" (Math|Float|Lerp (Variables|Default|GetTurnedOffIntensity) (Variables|Default|GetTurnedOnIntensity) _timetoon)))
    (:Finished
      (Variables|Default|SetIsPowered true))))

(event EventOnPowerOff
  (Default|CallDecrementPuzzleCounter)
  (bind _timetooff (Timeline|TimeToOff PlayFromStart)
    (:Update
      (Rendering|Material|SetScalarParameterValueonMaterials (Variables|Default|GetStaticMesh) "emissive intensity" (Math|Float|Lerp (Variables|Default|GetTurnedOnIntensity) (Variables|Default|GetTurnedOffIntensity) _timetooff)))
    (:Finished
      (Variables|Default|SetIsPowered false))))

(fn ConstructionScript)

(fn TurnonOff
  (Utilities|FlowControl|FlipFlop
    (:A
      (Rendering|Material|SetScalarParameterValueonMaterials (Variables|Default|GetStaticMesh) "emissive intensity" 0.0))
    (:B
      (Rendering|Material|SetScalarParameterValueonMaterials (Variables|Default|GetStaticMesh) "emissive intensity" 0.15))))

(fn GetGlyphProvider
  (return 0))