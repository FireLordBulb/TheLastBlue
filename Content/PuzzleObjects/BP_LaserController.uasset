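; Puzzle controller that lets glyph sentences entered on a Display switch a laser and an elevator on and off.
; On BeginPlay it registers start and stop sentences with the Display's glyph provider, toggling SingleLaser and MoveControllerRef and swapping indicator mesh materials blue or red.
; When the move controller stops, it powers down the laser wall, lights the power indicator and turns the meshes blue.
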(event Custom|SendPowerToLaser
  (CallFunction|PowerUpLaser)
  (CallFunction|FlipMeshtoBlue)
  (CallFunction|PowerUpIndicator)
  (CallFunction|PowerElevator))

(event Custom|CutPowerToLaser
  (CallFunction|PowerDownLaser)
  (CallFunction|FlipMeshtoRed)
  (CallFunction|UnpowerElevator))

(event Custom|DeactivateLaserWall
  (CallFunction|PowerDownLaserWall)
  (CallFunction|PowerUpIndicator)
  (CallFunction|FlipMeshtoBlue))

(event EventBeginPlay
  (bind _display (Variables|Default|GetDisplay))
  (Utilities|IsValid _display
    (:Is%20Valid
      (bind _glyphprovider (Default|GetGlyphProvider _display))
      (Class|GlyphProvider|RegisterGlyphResponse _glyphprovider (Variables|Default|GetStartSentence) (delegate Custom|SendPowerToLaser))
      (Class|GlyphProvider|RegisterGlyphResponse _glyphprovider (Variables|Default|GetStopSentence) (delegate Custom|CutPowerToLaser))
      (EventDispatchers|BindEventtoOnMovementStop (Variables|Default|GetMoveControllerRef) (delegate Custom|DeactivateLaserWall)))))

(fn ConstructionScript)

(fn PowerDownLaserWall
  (for _array_element (Variables|Default|GetLasersToPower)
    (Default|OnPowerOff _array_element)))

(fn PowerUpLaserWall
  (for _array_element (Variables|Default|GetLasersToPower)
    (Default|OnPoweron _array_element)))

(fn FlipMeshtoRed
  (for _array_element (Variables|Default|GetMeshesToFlipBetweenR&B)
    (Rendering|Material|SetMaterial (Variables|/Script/Engine.StaticMeshActor|GetStaticMeshComponent _array_element) 0 "/Game/Materials/BlockOut_Materials/M_ED_Lv1PrototypeProgressIndicator_Inst3.M_ED_Lv1PrototypeProgressIndicator_Inst3")))

(fn FlipMeshtoBlue
  (for _array_element (Variables|Default|GetMeshesToFlipBetweenR&B)
    (Rendering|Material|SetMaterial (Variables|/Script/Engine.StaticMeshActor|GetStaticMeshComponent _array_element) 0 "/Game/Materials/BlockOut_Materials/M_ED_Lv1PrototypeProgressIndicator_Inst4.M_ED_Lv1PrototypeProgressIndicator_Inst4")))

(fn PowerUpIndicator
  (Default|OnPoweron (Variables|Default|GetPowerIndicator)))

(fn PowerDownIndicator
  (Default|OnPowerOff (Variables|Default|GetPowerIndicator)))

(fn PowerElevator
  (bind _movecontrollerref (Variables|Default|GetMoveControllerRef))
  (Utilities|IsValid _movecontrollerref
    (:Is%20Valid
      (Default|OnPoweron _movecontrollerref))))

(fn UnpowerElevator
  (bind _movecontrollerref (Variables|Default|GetMoveControllerRef))
  (Utilities|IsValid _movecontrollerref
    (:Is%20Valid
      (Default|OnPowerOff _movecontrollerref))))

(fn PowerDownLaser
  (bind _singlelaser (Variables|Default|GetSingleLaser))
  (Utilities|IsValid _singlelaser
    (:Is%20Valid
      (Default|OnPowerOff _singlelaser))))

(fn PowerUpLaser
  (bind _singlelaser (Variables|Default|GetSingleLaser))
  (Utilities|IsValid _singlelaser
    (:Is%20Valid
      (Default|OnPoweron _singlelaser))))