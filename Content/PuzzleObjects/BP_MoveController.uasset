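; Puzzle controller that shuttles a target actor between start and end transforms when its glyph forms the expected sentence.
; It registers a response with the GlyphProvider, starts only while powered, and moves the actor on Tick, using a dot product to detect arrival.
; During travel it disables glyph interaction and swaps invisible wall collision.
; On arrival it reverses direction, resets the glyph word with a temporary material fix, and signals the stop.
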(event Custom|StartMovingEvent
  ;[0.1643 0.6834 1] Register Delegates to GlyphProvider
  (CallFunction|StartMoving))

(event EventOnPoweron
  ;[1 0.915 0.083] Power on/off
  (Variables|Default|SetIsPowered true))

(event EventOnPowerOff
  ;[1 0.915 0.083] Power on/off
  (Variables|Default|SetIsPowered false))

(event EventTick
  (params (DeltaSeconds :type Float%20%28single-precision%29))
  (bind _controllingglyph (Variables|Default|GetControllingGlyph))
  (bind _resetword (Variables|Default|GetResetWord))
  (bind _returnvalue (Actor|GetComponentbyClass _controllingglyph "/Script/GP3_Team09.Interaction"))
  ;[0.1249 1 0.9901] Moving the actor each frame
  (if (Variables|Default|GetIsMoving)
    (bind _output_get (Variables|Default|SetCurrentSpeed (Utilities|CalculateNewSpeed DeltaSeconds)))
    (Transformation|AddActorWorldOffset (Variables|Default|GetTargetActor) (* _output_get DeltaSeconds (Variables|Default|GetDirection)))
    (Math|Float|CompareFloat 0.0 (Math|Vector|DotProduct (- (Variables|Default|GetTargetPosition) (Transformation|GetActorLocation (Variables|Default|GetTargetActor))) (Variables|Default|GetDirection))
      (:>
        _)
      (:==
        _))
    ;[0.7375 1 0.195] Set values when the target position is reached to make the next move go in reverse
    (Variables|Default|SetIsMoving false)
    (Transformation|SetActorLocation (Variables|Default|GetTargetActor) (Variables|Default|GetTargetPosition) false false)
    (bind _output_get_2 (Variables|Default|SetIsAtStart (not (Variables|Default|GetIsAtStart))))
    (Variables|Default|SetTargetPosition (Math|Vector|SelectVector (Transformation|GetWorldLocation (Variables|Default|GetEndTransform)) (Transformation|GetWorldLocation (Variables|Default|GetStartTransform)) _output_get_2))
    (Variables|Default|SetDirection (* (Variables|Default|GetDirection) -1.0))
    (Variables|Default|SetCurrentSpeed 0.0)
    (CallFunction|SetInvisibleWallEnableCollision false)
    ;[1 0.1238 0.1039] Resetting the Glyph when movement is over.
    (Class|GlyphProvider|SetMinorGlyph (Variables|Default|GetGlyphProvider) 0 (.position _resetword) (.word _resetword))
    (Utilities|IsValid _returnvalue
      (:Is%20Valid
        (Class|Interaction|SetEnabled _returnvalue true))
      (:Is%20Not%20Valid
        _))
    ;[1 0 1] Temporary solution. Won't be needed when changing the minor glyph will refresh the generated texure on the whole glyph.
    (CallFunction|SetSubglyphSymbolTEMP)
    (Default|CallOnMovementStop)))

(event EventBeginPlay
  (bind _targetactor (Variables|Default|GetTargetActor))
  (bind _controllingglyph (Variables|Default|GetControllingGlyph))
  (bind _returnvalue (Actor|GetComponentbyClass _controllingglyph "/Script/SentenceBuilder.GlyphProvider"))
  ;[0.1 0.205 1] Setup the first move from StartTransform to EndTransform
  (Utilities|IsValid _targetactor
    (:Is%20Valid
      (Transformation|SetWorldLocation (Variables|Default|GetStartTransform) (Transformation|GetActorLocation _targetactor) false false)
      (Variables|Default|SetDirection (Class|KismetMathLibrary|VectorNormalUnsafe (- (Transformation|GetWorldLocation (Variables|Default|GetEndTransform)) (Transformation|GetWorldLocation (Variables|Default|GetStartTransform)))))
      (Variables|Default|SetTargetPosition (Transformation|GetWorldLocation (Variables|Default|GetEndTransform)))
      (CallFunction|SetInvisibleWallEnableCollision false)
      ;[0.1643 0.6834 1] Register Delegates to GlyphProvider
      (Utilities|IsValid _controllingglyph
        (:Is%20Valid
          (Utilities|IsValid _returnvalue
            (:Is%20Valid
              (bind _output_get (Variables|Default|SetGlyphProvider _returnvalue))
              (Class|GlyphProvider|RegisterGlyphResponse _output_get (Variables|Default|GetMoveSentence) (delegate Custom|StartMovingEvent)))
            (:Is%20Not%20Valid
              (Development|PrintString "Glyph doesn't have a GlyphProvider!!"))))
        (:Is%20Not%20Valid
          (Development|PrintString "MoveController doesn't have Glyph reference!"))))
    (:Is%20Not%20Valid
      (Utilities|String|LogString "Target actor was not initialized in MoveController"))))

(fn ConstructionScript)

(fn StartMoving
  (bind _controllingglyph (Variables|Default|GetControllingGlyph))
  (bind _returnvalue (Actor|GetComponentbyClass _controllingglyph "/Script/GP3_Team09.Interaction"))
  (if (Variables|Default|GetIsPowered)
    (Variables|Default|SetIsMoving true)
    (CallFunction|SetInvisibleWallEnableCollision true)
    (Utilities|IsValid _returnvalue
      (:Is%20Valid
        (Class|Interaction|SetEnabled _returnvalue false)))))

(fn SetSubglyphSymbolTEMP
  (bind _resetword (Variables|Default|GetResetWord))
  (for _array_element (Actor|GetComponentsByClass (Variables|Default|GetControllingGlyph) "/Script/GP3_Team09.SubGlyph")
    (for (_array_element_2 _array_index) (Variables|/Script/GP3_Team09.SubGlyph|GetSymbols _array_element)
      (if (and (Utilities|Enum|Equal(Enum) (.word _array_element_2) (.word _resetword)) (Utilities|Enum|Equal(Enum) (.position _array_element_2) (.position _resetword)))
        (bind _asbp_base_glyph (Utilities|Casting|CastToBP_BaseGlyph (Variables|Default|GetControllingGlyph)))
        (Default|SetSubGlyphMaterial _asbp_base_glyph _array_element _array_index false)
        (return)))))

(fn SetInvisibleWallEnableCollision
  (params (NewEnableCollision :type Boolean))
  (bind _invisiblewallwhenmoving (Variables|Default|GetInvisibleWallWhenMoving))
  (for _array_element (Variables|Default|GetInvisibleWallsWhenNotMoving)
    (Collision|SetActorEnableCollision _array_element (not NewEnableCollision)))
  (Utilities|IsValid _invisiblewallwhenmoving
    (:Is%20Valid
      (Collision|SetActorEnableCollision _invisiblewallwhenmoving NewEnableCollision))))

(fn GetGlyphProvider
  (return (Variables|Default|GetGlyphProvider)))