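; Puzzle component that scales its owning actor between small, default and big sizes in response to sentences from a controlling glyph.
; It registers a response per size with the glyph's GlyphProvider, computing target scales from the owner's initial scale.
; Tick interpolates the scale with cosine easing.
; It is disabled while scaling, re-enabled on finishing only if small, and then asks any valid EnergySocket to recheck its power source's scale.
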(event Custom|MakeSmall
  ;[0.1643 0.6834 1] Register Delegates to GlyphProvider
  (Utilities|StartScaling (Variables|Default|GetSmallScale)))

(event Custom|MakeBig
  ;[0.1643 0.6834 1] Register Delegates to GlyphProvider
  (Utilities|StartScaling (Variables|Default|GetBigScale)))

(event Custom|MakeScaleDefault
  ;[0.1643 0.6834 1] Register Delegates to GlyphProvider
  (Utilities|StartScaling (Variables|Default|GetDefaultScale)))

(event EventBeginPlay
  (bind _controllingglyph (Variables|Default|GetControllingGlyph))
  (bind _returnvalue (Actor|GetComponentbyClass _controllingglyph "/Script/SentenceBuilder.GlyphProvider"))
  (|CallParentFunction)
  (bind _output_get (Variables|Default|SetOwningActor (Components|GetOwner)))
  (bind _output_get_2 (Variables|Default|SetDefaultScale (Class|Actor|GetActorRelativeScale3D _output_get)))
  (Variables|Default|SetTargetScale _output_get_2)
  (Variables|Default|SetSmallScale (* _output_get_2 (Variables|Default|GetSmallScaleMultiplier)))
  (Variables|Default|SetBigScale (* _output_get_2 (Variables|Default|GetBigScaleMultiplier)))
  ;[0.1643 0.6834 1] Register Delegates to GlyphProvider
  (Utilities|IsValid _controllingglyph
    (:Is%20Valid
      (Utilities|IsValid _returnvalue
        (:Is%20Valid
          (bind _output_get_3 (Variables|Default|SetGlyphProvider _returnvalue))
          (Class|GlyphProvider|RegisterGlyphResponse _output_get_3 (Variables|Default|GetSmallSentence) (delegate Custom|MakeSmall))
          (Class|GlyphProvider|RegisterGlyphResponse (Variables|Default|GetGlyphProvider) (Variables|Default|GetDefaultSentence) (delegate Custom|MakeScaleDefault))
          (Class|GlyphProvider|RegisterGlyphResponse (Variables|Default|GetGlyphProvider) (Variables|Default|GetBigSentence) (delegate Custom|MakeBig))
          (Class|GlyphProvider|ConfirmGlyph (Variables|Default|GetGlyphProvider)))
        (:Is%20Not%20Valid
          (Development|PrintString "Glyph doesn't have a GlyphProvider!!"))))))

(event EventTick
  (params (DeltaSeconds :type Float%20%28single-precision%29))
  (if (Variables|Default|GetIsScaling)
    (bind _output_get (Variables|Default|SetScalingTimeLeft (- (Variables|Default|GetScalingTimeLeft) DeltaSeconds)))
    (Math|Float|CompareFloat _output_get 0.0
      (:>
        _)
      (:==
        (Utilities|FinishScaling :!label _label))
      (:<
        (goto _label)))
    (Transformation|SetActorRelativeScale3D (Variables|Default|GetOwningActor) (Math|Vector|Lerp(Vector) (Variables|Default|GetPreviousScale) (Variables|Default|GetTargetScale) (Utilities|CalculateScaleAlpha)))))

(fn IsSmall
  (return (Utilities|IsScale (Variables|Default|GetSmallScale))))

(fn IsDefault
  (return (Utilities|IsScale (Variables|Default|GetDefaultScale))))

(fn IsBig
  (return (Utilities|IsScale (Variables|Default|GetBigScale))))