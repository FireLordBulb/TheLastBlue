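; BP_WaterDrainer is a puzzle object that changes the water level one time after it opens.
; When its animation finishes in the open state, it sets a one-shot flag and shifts the referenced WaterLevel by a configurable amount.
; It then hides the water spout's NS component and sends the spout a "FinishPlaying" trigger parameter message.
; BeginPlay and construction only call the parent.
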(event EventBeginPlay
  (|CallParentFunction))

(fn ConstructionScript
  (|CallParentFunction))

(fn OnAnimationFinished
  (bind _waterspout (Variables|Default|GetWaterSpout))
  (if (not (Variables|Default|GetHasDrainedOnce))
    (if (Variables|Default|GetIsOpen)
      (Variables|Default|SetHasDrainedOnce true)
      (Default|ChangeWaterLevelby (Variables|Default|GetWaterLevel) (Variables|Default|GetWaterChangeAmount))
      (Rendering|SetVisibility (Variables|/Game/Art/VFX/WaterSpout/NS/BP_WaterSpout.BP_WaterSpout_C|GetNS _waterspout) false false)
      (Class|AudioParameterControllerInterface|SetTriggerParameter(Message) _waterspout "FinishPlaying"))))

(fn GetGlyphProvider
  (return 0))