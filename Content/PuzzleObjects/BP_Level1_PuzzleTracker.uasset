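; BP_Level1_PuzzleTracker tracks how many power indicators are active in the Level 1 puzzle and controls the exit state.
; On BeginPlay it finds every BP_PowerIndicator tagged for Level 1 and binds to its increment and decrement counter events.
; When the count reaches four, it lights the final indicator, powers the last laser and opens the door.
; Dropping below four reverses all three.
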(event Custom|IncrementCount
  ;[1 1 1] Increments the count when "increment puzzle counter" event is fired on BP_PowerIndicators in the array
  (bind _result (Math|Integer|IncrementInt (Variables|Default|GetPowerCount))
    (:%20%20
      (if (>= _result 4)
        (Utilities|FlowControl|Sequence
          (:then_0
            ;[1 1 1] Lights up indicators and opens the door
            (Default|EventLightUp (Variables|Default|GetLastPowerIndicator)))
          (:then_1
            (Default|OnPoweron (Variables|Default|GetLastLaser)))
          (:then_2
            (Default|OpenDoor (Variables|Default|GetDoor))))))))

(event Custom|DecrementCount
  ;[1 1 1] Decrements the count when "decrement puzzle counter" event is fired on BP_PowerIndicators in the array
  (bind _result (Math|Integer|DecrementInt (Variables|Default|GetPowerCount))
    (:%20%20
      (if (<= _result 3)
        ;[1 1 1] Powers down indicators and closes the door
        (Utilities|FlowControl|Sequence
          (:then_0
            (Default|EventLightDown (Variables|Default|GetLastPowerIndicator)))
          (:then_1
            (Default|OnPowerOff (Variables|Default|GetLastLaser)))
          (:then_2
            (Default|CloseDoor (Variables|Default|GetDoor))))))))

(event EventBeginPlay
  (bind _outactors (Actor|GetAllActorsOfClasswithTag "/Game/PuzzleObjects/BP_PowerIndicator.BP_PowerIndicator_C" (Variables|Default|GetLevel1Tag)))
  (bind _output_get (Variables|Default|SetPowerIndicatorActorArray _outactors))
  (for _array_element _output_get
    (EventDispatchers|BindEventtoIncrementPuzzleCounter _array_element (delegate Custom|IncrementCount))
    (EventDispatchers|BindEventtoDecrementPuzzleCounter _array_element (delegate Custom|DecrementCount))))

(fn ConstructionScript)