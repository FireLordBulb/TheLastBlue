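; BP_PowerLine is a puzzle object that shows a power line turning on and off through an emissive glow on its Plane mesh.
; BeginPlay sets the "Emissive Strength" material parameter to the off intensity.
; LightUp and LightDown each play their own timeline, lerping that parameter between the off and on intensities.
; GetGlyphProvider is an empty stub, and the construction script does nothing.
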(event Custom|Event%20Light%20Up
  (bind _timetoon (Timeline|Timeline Play)
    (:Update
      (Rendering|Material|SetScalarParameterValueonMaterials (Variables|Default|GetPlane) "Emissive Strength" (Math|Float|Lerp (Variables|Default|GetTurnedOffIntensity) (Variables|Default|GetTurnedOnIntensity) _timetoon)))))

(event Custom|Event%20Light%20Down
  (bind _timetooff (Timeline|Timeline_0 Play)
    (:Update
      (Rendering|Material|SetScalarParameterValueonMaterials (Variables|Default|GetPlane) "Emissive Strength" (Math|Float|Lerp (Variables|Default|GetTurnedOnIntensity) (Variables|Default|GetTurnedOffIntensity) _timetooff)))))

(event EventBeginPlay
  (CallFunction|InitEmissive))

(fn ConstructionScript)

(fn InitEmissive
  (Rendering|Material|SetScalarParameterValueonMaterials (Variables|Default|GetPlane) "Emissive Strength" (Variables|Default|GetTurnedOffIntensity)))

(fn GetGlyphProvider
  (return 0))