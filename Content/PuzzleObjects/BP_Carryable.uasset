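; BP_Carryable is an interaction component that lets the player character pick up and put down its owning actor.
; It enables itself from StartsCarryable at BeginPlay, then on each interaction toggles its priority and passes the owner to the player's CarryInteraction.
; The returned result hides or shows the spawned widget, and when shown, the interaction is removed if the player no longer overlaps the collision mesh.
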(event Custom|CarryInteraction
  (bind _instancespawnwidget (Variables|Default|GetInstanceSpawnWidget))
  (bind _returnvalue (UserInterface|GetUserWidgetObject _instancespawnwidget))
  (Variables|Default|SetbIsPriority (not (Variables|Default|GetbIsPriority)))
  (bind _asbp_player_character (Utilities|Casting|CastToBP_PlayerCharacter (Game|Player|GetPlayerPawn 0)))
  (bind _iscarried (Default|CarryInteraction _asbp_player_character (Components|GetOwner)))
  (if _iscarried
    (Variables|/Script/UMG.Widget|SetVisibility _returnvalue "Collapsed")
    (else
      (Variables|/Script/UMG.Widget|SetVisibility _returnvalue "Visible")
      (if (Utilities|Array|IsEmpty (Collision|GetOverlappingActors (Variables|Default|GetCollisionMesh) "/Script/GP3_Team09.PlayerCharacter" :!class /Script/Engine.PrimitiveComponent))
        (Class|PlayerCharacterInteract|RemoveInteraction (Variables|Default|GetPlayerCharacterInteract) self)))))

(event EventBeginPlay
  (EventDispatchers|BindEventtoInteracted (delegate Custom|CarryInteraction))
  (Class|Interaction|SetEnabled (Variables|Default|GetStartsCarryable)))