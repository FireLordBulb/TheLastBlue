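; BP_EnergySocket is a puzzle socket that powers linked receivers when it holds an energy source of the desired scale.
; An overlapping BP_SmallBig energy source within SnappingRadius snaps in and gets its scale checked; ending overlap clears it and cuts power.
; BeginPlay resolves PowerReceivers from actor references or their components, working around unserializable interface references.
; Power changes notify receivers and light or dim PowerLines, with glyph confirmation on power-on.
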(event OnComponentBeginOverlap(SnappingCollision)
  (params (OverlappedComponent :type Primitive%20Component%20Object%20Reference) (OtherActor :type Actor%20Object%20Reference) (OtherComp :type Primitive%20Component%20Object%20Reference) (OtherBodyIndex :type Integer) (bFromSweep :type Boolean) (SweepResult :type Hit%20Result%20Structure%20%28by%20ref%29))
  (bind _returnvalue (Actor|GetComponentbyClass OtherActor "/Game/PuzzleObjects/BP_SmallBig.BP_SmallBig_C"))
  ;[0.1424 1 0.4272] Attaching an energy source
  (Utilities|IsValid (Variables|Default|GetEnergySource)
    (:Is%20Not%20Valid
      (Utilities|IsValid _returnvalue
        (:Is%20Valid
          (if (Variables|/Game/PuzzleObjects/BP_SmallBig.BP_SmallBig_C|GetIsEnergySource _returnvalue)
            (Math|Float|CompareFloat (Variables|Default|GetSnappingRadius) (Math|Vector|Distance(Vector) (Transformation|GetActorLocation OtherActor) (Transformation|GetWorldLocation (Variables|Default|GetEnergySourceTransform)))
              (:>
                _)
              (:==
                _))
            (bind _output_get (Variables|Default|SetEnergySource _returnvalue))
            (Variables|/Game/PuzzleObjects/BP_SmallBig.BP_SmallBig_C|SetEnergySocket _output_get self)
            (Transformation|AttachComponentToComponent OtherActor (Variables|Default|GetEnergySourceTransform) "None" "SnapToTarget" "KeepRelative" "KeepRelative" false)
            (CallFunction|CheckPowerSourceScale)))))))

(event OnComponentEndOverlap(SnappingCollision)
  (params (OverlappedComponent :type Primitive%20Component%20Object%20Reference) (OtherActor :type Actor%20Object%20Reference) (OtherComp :type Primitive%20Component%20Object%20Reference) (OtherBodyIndex :type Integer))
  ;[1 0.4305 0.2598] Removing the energy source
  (Utilities|IsValid (Variables|Default|GetEnergySource)
    (:Is%20Valid
      (if (== OtherActor (Components|GetOwner (Variables|Default|GetEnergySource)))
        (Variables|/Game/PuzzleObjects/BP_SmallBig.BP_SmallBig_C|SetEnergySocket (Variables|Default|GetEnergySource) 0)
        (Variables|Default|SetEnergySource 0)
        (CallFunction|PowerOff)))))

(event EventBeginPlay
  ;[0.9067 1 0.3036] Casting Actors/components to PowerReceiver interface because you can't serialize references to interfaces in a level in Unreal. Pain.
  (for _array_element (Variables|Default|GetPowerReceivingActors)
    (bind _aspower_receiver (Utilities|Casting|CastToPowerReceiver _array_element)
      (:then
        (Utilities|Array|Add (Variables|Default|GetPowerReceivers) _aspower_receiver))
      (:CastFailed
        (for _array_element_2 (Class|Actor|GetComponentsbyInterface _array_element "/Script/GP3_Team09.PowerReceiver")
          (bind _aspower_receiver_2 (Utilities|Casting|CastToPowerReceiver _array_element_2))
          (Utilities|Array|Add (Variables|Default|GetPowerReceivers) _aspower_receiver_2))))))

(fn ConstructionScript)

(fn Poweron
  (bind _powerlines (Variables|Default|GetPowerLines))
  (if (not (Variables|Default|GetPowerIsOn))
    (Variables|Default|SetPowerIsOn true)
    (for _array_element (Variables|Default|GetPowerReceivers)
      (Class|PowerReceiver|OnPoweron _array_element)
      (bind _returnvalue (Class|PowerReceiver|GetGlyphProvider _array_element))
      (Utilities|IsValid _returnvalue
        (:Is%20Valid
          (bind _asglyph_provider (Utilities|Casting|CastToGlyphProvider _returnvalue))
          (Class|GlyphProvider|ConfirmGlyph _asglyph_provider)
          (if (Utilities|Array|IsNotEmpty _powerlines)
            (for _array_element_2 _powerlines
              (Default|EventLightUp _array_element_2))))))
    (Development|PrintString "Power turned on!")))

(fn PowerOff
  (bind _powerlines (Variables|Default|GetPowerLines))
  (if (Variables|Default|GetPowerIsOn)
    (Variables|Default|SetPowerIsOn false)
    (for _array_element (Variables|Default|GetPowerReceivers)
      (Class|PowerReceiver|OnPowerOff _array_element)
      (if (Utilities|Array|IsNotEmpty _powerlines)
        (for _array_element_2 _powerlines
          (Default|EventLightDown _array_element_2))))
    (Development|PrintString "Power turned off!")))

(fn CheckPowerSourceScale
  (bind _energysource (Variables|Default|GetEnergySource))
  (if (Utilities|Select :Index (Variables|Default|GetDesiredScaleIndex) :Option%200 (Default|IsSmall _energysource) :Option%201 (Default|IsDefault _energysource) :Option%202 (Default|IsBig _energysource))
    (CallFunction|Poweron)
    (Audio|SpawnSoundatLocation "/Game/Audio/SFX/OneShots/WAVs/SFX_PowerOnOS.SFX_PowerOnOS" (+ (Transformation|GetWorldLocation (Variables|Default|GetEnergySourceTransform)) "0.000000,0.000000,50.000000") "0, 0, 0" 1.0 1.0 0.0 0 0)
    (else
      (CallFunction|PowerOff))))