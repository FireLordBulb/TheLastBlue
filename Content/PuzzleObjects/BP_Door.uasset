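; BP_Door is a puzzle door that slides open and closed in response to glyph sentences, but only while powered.
; On BeginPlay it registers open and close responses with the GlyphProvider component of its controlling glyph and applies any initial open state.
; Timelines lerp the door mesh parent by a relative offset, negated for closing.
; A moving sound starts with each slide and receives a finish trigger when the animation ends.
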(event Custom|OpenDoor
  ;[1 1 1] Open Door
  (if (and (not (Variables|Default|GetIsOpen)) (Variables|Default|GetIsPowered))
    (Utilities|TryStartAnimation false)
    (bind _returnvalue (Audio|SpawnSoundatLocation (Variables|Default|GetSound) (Variables|Default|GetDoorTargetPosition) "0, 0, 0" 1.0 1.0 0.0 0 0))
    (Variables|Default|SetSFX _returnvalue)
    (bind _animation (Timeline|Timeline PlayFromStart)
      (:Update
        (Utilities|AnimationUpdate _animation))
      (:Finished
        (Utilities|AnimationFinished)))))

(event Custom|CloseDoor
  ;[1 1 1] Close Door
  (if (and (Variables|Default|GetIsOpen) (Variables|Default|GetIsPowered))
    (Utilities|TryStartAnimation true)
    (bind _returnvalue (Audio|SpawnSoundatLocation "/Game/Audio/SFX/OneShots/MetaSoundSources/MSS_DoorMoving.MSS_DoorMoving" (Variables|Default|GetDoorTargetPosition) "0, 0, 0" 1.0 1.0 0.0 0 0))
    (Variables|Default|SetSFX _returnvalue)
    (bind _animation (Timeline|Timeline_0 PlayFromStart)
      (:Update
        (Utilities|AnimationUpdate _animation))
      (:Finished
        (Utilities|AnimationFinished)))))

(event EventOnPoweron
  ;[1 0.915 0.083] Power on/off
  (Variables|Default|SetIsPowered true))

(event EventOnPowerOff
  ;[1 0.915 0.083] Power on/off
  (Variables|Default|SetIsPowered false))

(event EventBeginPlay
  (bind _controllingglyph (Variables|Default|GetControllingGlyph))
  (bind _returnvalue (Actor|GetComponentbyClass _controllingglyph "/Script/SentenceBuilder.GlyphProvider"))
  (CallFunction|SetupStartPosition)
  ;[0.1643 0.6834 1] Register Delegates to GlyphProvider
  (Utilities|IsValid _controllingglyph
    (:Is%20Valid
      (Utilities|IsValid _returnvalue
        (:Is%20Valid
          (bind _output_get (Variables|Default|SetGlyphProvider _returnvalue))
          (Class|GlyphProvider|RegisterGlyphResponse _output_get (Variables|glyphControl|GetOpenSentence) (delegate Custom|OpenDoor))
          (Class|GlyphProvider|RegisterGlyphResponse (Variables|Default|GetGlyphProvider) (Variables|GlyphControl|GetCloseSentence) (delegate Custom|CloseDoor)))
        (:Is%20Not%20Valid
          (Development|PrintString "Glyph doesn't have a GlyphProvider!!"))))))

(fn ConstructionScript)

(fn SetupStartPosition
  (if (Variables|Default|GetIsOpen)
    (Utilities|TryStartAnimation false)
    (Utilities|AnimationUpdate 1.0
      (:Exec
        (Variables|Default|SetIsAnimationPlaying false)))))

(fn OnAnimationFinished)

(fn GetGlyphProvider
  (return (Variables|Default|GetGlyphProvider)))