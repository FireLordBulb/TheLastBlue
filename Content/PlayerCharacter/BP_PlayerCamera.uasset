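; Player camera component that glides between attach targets and can return to a default parent, initially the one it starts attached to.
; Setting a target reattaches it to that scene component while keeping world location and rotation, then starts movement.
; Tick lerps the world transform toward the target with a frame-time-scaled alpha, using a distance-based minimum speed so it finishes instead of endlessly easing.
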(event EventBeginPlay
  (Variables|Default|SetDefault%20Parent%20Transform (Transformation|GetAttachParent))
  (CallFunction|ReturntoPlayer))

(event EventTick
  (params (DeltaSeconds :type Float%20%28single-precision%29))
  (bind _returnvalue (Transformation|GetWorldLocation))
  (bind _target_transform (Variables|Default|GetTarget%20Transform))
  (bind _returnvalue_2 (Transformation|GetWorldLocation _target_transform))
  (bind _returnvalue_3 (Math|Vector|Distance(Vector) _returnvalue _returnvalue_2))
  (bind _alpha (CallFunction|CalculateLerpAlpha DeltaSeconds _returnvalue_3))
  ;[0.1892 1 0.7257] Position and Rotation lerping toward the target transform
  (if (Variables|Default|GetIsMoving)
    (Variables|Default|SetIsMoving (< _alpha 1.0))
    (Transformation|SetWorldTransform (Math|Transform|Lerp(Transform) (Transformation|GetWorldTransform) (Transformation|GetWorldTransform _target_transform) _alpha) false false)))

(fn SetTargetTransform
  (params (Transform :type Scene%20Component%20Object%20Reference))
  (Variables|Default|SetPrevious%20Parent%20Transform (Transformation|GetAttachParent))
  (bind _output_get (Variables|Default|SetTarget%20Transform Transform))
  (Transformation|AttachComponentToComponent _output_get "None" "KeepWorld" "KeepWorld" "KeepRelative" false)
  (Variables|Default|SetIsMoving true))

(fn ReturntoPlayer
  (CallFunction|SetTargetTransform (Variables|Default|GetDefault%20Parent%20Transform)))

(fn CalculateLerpAlpha
  (params (DeltaSeconds :type Float%20%28double-precision%29) (DistanceLeft :type Float%20%28double-precision%29))
  (return (Math|Float|Clamp(Float) (* DeltaSeconds (Math|Float|Max(Float) (/ (Variables|Default|GetMin%20Speed) (Math|Float|Max(Float) DistanceLeft 0.001)) (Variables|Default|GetLerp%20Alpha%20Per%20Second))))))

(fn SetDefaultParent
  (params (SceneComponent :type Scene%20Component%20Object%20Reference))
  (Variables|Default|SetDefault%20Parent%20Transform SceneComponent)
  (CallFunction|ReturntoPlayer))

(fn GetDefaultParent
  (return (Variables|Default|GetDefault%20Parent%20Transform)))