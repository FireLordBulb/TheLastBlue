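; Player interaction component for BP_PlayerCharacter that routes the GlyphInteract, Interact and Point inputs to the closest interaction of the matching type.
; Glyph interaction is blocked while carrying or in the journal, and switches input mode and mouse capture with glyph editing.
; Interact redirects to the glyph path during editing.
; Point can send the target's held sentence to the journal as a spirit sentence.
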(event Input|EnhancedActionEvents|EnhancedInputActionIA_Interact
  (params (ActionValue :type Boolean) (ElapsedSeconds :type Float%20%28double-precision%29) (TriggeredSeconds :type Float%20%28double-precision%29) (InputAction :type Input%20Action%20Object%20Reference :default "/Game/Input/IA_Interact.IA_Interact"))
  (bind _returnvalue (Class|PlayerCharacterInteract|GetClosestInteraction "Glyph"))
  (bind _returnvalue_2 (Class|PlayerCharacterInteract|GetClosestInteraction "Regular"))
  ;[1 0.1249 0.2547] Interact
  (:Triggered
    (if (Variables|/Script/GP3_Team09.PlayerGlyphEditor|GetbGlyphEditingIsActive (Variables|/Game/PlayerCharacter/BP_PlayerCharacter.BP_PlayerCharacter_C|GetBP_PlayerGlyphEditor (Variables|Default|GetPlayer)))
      ;[0.3894 0.09903 1] GlyphInteract
      (if (not (or (Variables|/Game/PlayerCharacter/BP_PlayerCharacter.BP_PlayerCharacter_C|GetIsCarrying (Variables|Default|GetPlayer)) (Variables|/Game/PlayerCharacter/BP_JournalToggler.BP_JournalToggler_C|GetIsJournalActive (Variables|/Game/PlayerCharacter/BP_PlayerCharacter.BP_PlayerCharacter_C|GetBP_JournalToggler (Variables|Default|GetPlayer)))))
        (Utilities|IsValid _returnvalue
          (:Is%20Valid
            (Class|Interaction|GlyphInteract _returnvalue)
            (if (Variables|/Script/GP3_Team09.PlayerGlyphEditor|GetbGlyphEditingIsActive (Variables|/Game/PlayerCharacter/BP_PlayerCharacter.BP_PlayerCharacter_C|GetBP_PlayerGlyphEditor (Variables|Default|GetPlayer)))
              (bind _asa_interactive_glyph_display (Utilities|Casting|CastToA_InteractiveGlyphDisplay (Components|GetOwner _returnvalue)))
              (bind _output_get (Variables|Default|SetExamine%20Interaction%20Widget (Variables|/Game/Glyphs/A_InteractiveGlyphDisplay.A_InteractiveGlyphDisplay_C|GetExamineInteractionWidget _asa_interactive_glyph_display)))
              (Input|SetInputModeGameandUI (Game|GetPlayerController 0) _output_get "DoNotLock" false false)
              (else
                (Input|SetInputModeGameOnly (Game|GetPlayerController 0) false)
                (Class|GameplayStatics|SetViewportMouseCaptureMode "CapturePermanently_IncludingInitialMouseDown") ; Ensures mouse input is always captured by IA_ScreenClick even when the mouse is visible (because of Glyph Editing) after unpausing.
              )))))
      (else
        (Utilities|IsValid _returnvalue_2
          (:Is%20Valid
            (Class|Interaction|Interact _returnvalue_2)))))))

(event Input|EnhancedActionEvents|EnhancedInputActionIA_Point
  (params (ActionValue :type Boolean) (ElapsedSeconds :type Float%20%28double-precision%29) (TriggeredSeconds :type Float%20%28double-precision%29) (InputAction :type Input%20Action%20Object%20Reference :default "/Game/Input/IA_Point.IA_Point"))
  (bind _returnvalue (Class|PlayerCharacterInteract|GetClosestInteraction "Point"))
  ;[1 0.5311 0.5411] Point
  (:Started
    (Utilities|IsValid _returnvalue
      (:Is%20Valid
        (Class|Interaction|Point _returnvalue)
        (if (Variables|/Script/GP3_Team09.Interaction|GetCanPointToSpirit _returnvalue)
          (Default|MakeSpiritSentence (Variables|/Game/PlayerCharacter/BP_JournalToggler.BP_JournalToggler_C|GetJournalWidget (Variables|/Game/PlayerCharacter/BP_PlayerCharacter.BP_PlayerCharacter_C|GetBP_JournalToggler (Variables|Default|GetPlayer))) (Variables|/Script/GP3_Team09.Interaction|GetHeldSentence _returnvalue)))))))

(event Input|EnhancedActionEvents|EnhancedInputActionIA_GlyphInteract
  (params (ActionValue :type Boolean) (ElapsedSeconds :type Float%20%28double-precision%29) (TriggeredSeconds :type Float%20%28double-precision%29) (InputAction :type Input%20Action%20Object%20Reference :default "/Game/Input/IA_GlyphInteract.IA_GlyphInteract"))
  (bind _returnvalue (Class|PlayerCharacterInteract|GetClosestInteraction "Glyph"))
  ;[0.3894 0.09903 1] GlyphInteract
  (:Triggered
    (if (not (or (Variables|/Game/PlayerCharacter/BP_PlayerCharacter.BP_PlayerCharacter_C|GetIsCarrying (Variables|Default|GetPlayer)) (Variables|/Game/PlayerCharacter/BP_JournalToggler.BP_JournalToggler_C|GetIsJournalActive (Variables|/Game/PlayerCharacter/BP_PlayerCharacter.BP_PlayerCharacter_C|GetBP_JournalToggler (Variables|Default|GetPlayer)))))
      (Utilities|IsValid _returnvalue
        (:Is%20Valid
          (Class|Interaction|GlyphInteract _returnvalue)
          (if (Variables|/Script/GP3_Team09.PlayerGlyphEditor|GetbGlyphEditingIsActive (Variables|/Game/PlayerCharacter/BP_PlayerCharacter.BP_PlayerCharacter_C|GetBP_PlayerGlyphEditor (Variables|Default|GetPlayer)))
            (bind _asa_interactive_glyph_display (Utilities|Casting|CastToA_InteractiveGlyphDisplay (Components|GetOwner _returnvalue)))
            (bind _output_get (Variables|Default|SetExamine%20Interaction%20Widget (Variables|/Game/Glyphs/A_InteractiveGlyphDisplay.A_InteractiveGlyphDisplay_C|GetExamineInteractionWidget _asa_interactive_glyph_display)))
            (Input|SetInputModeGameandUI (Game|GetPlayerController 0) _output_get "DoNotLock" false false)
            (else
              (Input|SetInputModeGameOnly (Game|GetPlayerController 0) false)
              (Class|GameplayStatics|SetViewportMouseCaptureMode "CapturePermanently_IncludingInitialMouseDown") ; Ensures mouse input is always captured by IA_ScreenClick even when the mouse is visible (because of Glyph Editing) after unpausing.
            )))))))

(event EventBeginPlay
  (bind _asbp_player_character (Utilities|Casting|CastToBP_PlayerCharacter (Components|GetOwner)))
  (Variables|Default|SetPlayer _asbp_player_character))