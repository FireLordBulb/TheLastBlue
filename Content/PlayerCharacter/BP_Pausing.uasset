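; BP_Pausing is a component that opens the pause menu when its owner receives the pause input.
; On BeginPlay it caches the owner's BP_JournalToggler component and ignores the pause input while that component reports an animation playing.
; Otherwise it creates a new WBP_PauseMenu widget, shows the mouse cursor, switches input to UI only and pauses the game.
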(event Input|EnhancedActionEvents|EnhancedInputActionIA_PauseGame
  (params (ActionValue :type Boolean) (ElapsedSeconds :type Float%20%28double-precision%29) (TriggeredSeconds :type Float%20%28double-precision%29) (InputAction :type Input%20Action%20Object%20Reference :default "/Game/Input/IA_PauseGame.IA_PauseGame"))
  (bind _returnvalue (Game|GetPlayerController 0))
  (:Started
    (if (not (Default|IsAnimationPlaying (Variables|Default|GetJournalToggler)))
      (bind _returnvalue_2 (UserInterface|CreateWidget "/Game/UI/WBP_PauseMenu.WBP_PauseMenu_C"))
      (UserInterface|Viewport|AddtoViewport _returnvalue_2 2)
      (Variables|/Script/Engine.PlayerController|SetbShowMouseCursor _returnvalue true)
      (Input|SetInputModeUIOnly _returnvalue 0 "DoNotLock" false)
      (Game|SetGamePaused true))))

(event EventBeginPlay
  (Variables|Default|SetJournalToggler (Actor|GetComponentbyClass (Components|GetOwner) "/Game/PlayerCharacter/BP_JournalToggler.BP_JournalToggler_C")))