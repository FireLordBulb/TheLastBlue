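; BP_JournalToggler is a player component that opens and closes the journal widget on the IA_Journal input.
; BeginPlay creates the collapsed journal and a hidden addition-notice widget; toggling is blocked while the journal animates or glyph editing is active.
; The journal animation plays forward or in reverse, switching visibility, cursor and input mode, with a closing sound and permanent mouse capture restored on close.
; AddSentence shows and animates the notice, which opening the journal hides.
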(event Input|EnhancedActionEvents|EnhancedInputActionIA_Journal
  (params (ActionValue :type Boolean) (ElapsedSeconds :type Float%20%28double-precision%29) (TriggeredSeconds :type Float%20%28double-precision%29) (InputAction :type Input%20Action%20Object%20Reference :default "/Game/Input/IA_Journal.IA_Journal"))
  (bind _returnvalue (Game|GetPlayerController 0))
  (bind _returnvalue_2 (Game|GetPlayerController 0))
  (:Started
    (if (not (or (CallFunction|IsAnimationPlaying) (Variables|/Script/GP3_Team09.PlayerGlyphEditor|GetbGlyphEditingIsActive (Variables|Default|GetPlayerGlyphEditor))))
      (if (Variables|Default|GetIsJournalActive)
        (Utilities|PlayJournalAnimation "Reverse"
          (:On%20Start
            (Audio|SpawnSound2D "/Game/Audio/SFX/OneShots/MetaSoundSources/MSS_CloseJournal.MSS_CloseJournal" 1.0 1.0 0.0 0)
            (Variables|/Script/Engine.PlayerController|SetbShowMouseCursor _returnvalue false)
            (Input|SetInputModeGameOnly _returnvalue false)
            (Class|GameplayStatics|SetViewportMouseCaptureMode "CapturePermanently_IncludingInitialMouseDown") ; Ensures mouse input is always captured by IA_ScreenClick even when the mouse is visible (because of Glyph Editing) after unpausing.
          )
          (:Finished
            (Widget|SetVisibility (Variables|Default|GetJournalWidget) "Collapsed")
            (Variables|Default|SetIsJournalActive false)))
        (else
          (Utilities|PlayJournalAnimation "Forward"
            (:On%20Start
              (Widget|SetVisibility (Variables|Default|GetJournalWidget) "Visible")
              (Variables|Default|SetIsJournalActive true)
              (CallFunction|RemoveAnimation))
            (:Finished
              (Variables|/Script/Engine.PlayerController|SetbShowMouseCursor _returnvalue_2 true)
              (Input|SetInputModeGameandUI _returnvalue_2 (Variables|Default|GetJournalWidget) "DoNotLock" false false))))))))

(event EventBeginPlay
  (bind _returnvalue (UserInterface|CreateWidget "/Game/Prototypes/WBP_JournalPrototype.WBP_JournalPrototype_C"))
  (bind _output_get (Variables|Default|SetJournalWidget _returnvalue))
  (UserInterface|Viewport|AddtoViewport _output_get 0)
  (Widget|SetVisibility _output_get "Collapsed")
  (Variables|Default|SetJournalAnimation (Variables|/Game/Prototypes/WBP_JournalPrototype.WBP_JournalPrototype_C|GetJournalAnimation _output_get))
  (Variables|Default|SetPlayerGlyphEditor (Actor|GetComponentbyClass (Components|GetOwner) "/Game/PlayerCharacter/BP_PlayerGlyphEditor.BP_PlayerGlyphEditor_C"))
  (bind _returnvalue_2 (UserInterface|CreateWidget "/Game/UI/WBP_JournalAddition.WBP_JournalAddition_C"))
  (bind _output_get_2 (Variables|Default|SetJournalAddition _returnvalue_2))
  (UserInterface|Viewport|AddtoViewport _output_get_2 0)
  (Variables|/Script/UMG.Widget|SetVisibility _output_get_2 "Hidden"))

(fn IsAnimationPlaying
  (return (Class|UserWidget|IsAnimationPlaying (Variables|Default|GetJournalWidget) (Variables|Default|GetJournalAnimation))))

(fn AddSentence
  (bind _journaladdition (Variables|Default|GetJournalAddition))
  (Variables|/Script/UMG.Widget|SetVisibility _journaladdition "Visible")
  (UserInterface|Animation|PlayAnimation _journaladdition (Variables|/Game/UI/WBP_JournalAddition.WBP_JournalAddition_C|GetUpdateAnimation _journaladdition) 0.0 1 "Forward" 1.0 false))

(fn RemoveAnimation
  (Variables|/Script/UMG.Widget|SetVisibility (Variables|Default|GetJournalAddition) "Hidden"))