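; BP_Checkpoint is a save checkpoint that writes game progress when the player character overlaps its sphere.
; The overlap pulls player data from the character and, if its Spirit reference is valid, spirit data from that Spirit.
; It passes each to the Game Instance through save messages, then triggers a journal save, all with Async set to false.
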(event OnComponentBeginOverlap(Sphere)
  (params (OverlappedComponent :type Primitive%20Component%20Object%20Reference) (OtherActor :type Actor%20Object%20Reference) (OtherComp :type Primitive%20Component%20Object%20Reference) (OtherBodyIndex :type Integer) (bFromSweep :type Boolean) (SweepResult :type Hit%20Result%20Structure%20%28by%20ref%29))
  (bind _spirit (Variables|Default|GetSpirit))
  (bind _asbp_player_character (Utilities|Casting|CastToBP_PlayerCharacter OtherActor))
  (bind _player_save_data (Default|GetPlayerData _asbp_player_character))
  (Class|BPISaveGame|SavePlayerData(Message) (Game|GetGameInstance) _player_save_data false)
  (Utilities|IsValid _spirit
    (:Is%20Valid
      (bind _spirit_save_data (Default|GetSpiritData _spirit))
      (Class|BPISaveGame|SaveSpiritData(Message) (Game|GetGameInstance) _spirit_save_data false))
    (:Is%20Not%20Valid
      _))
  (Class|BPISaveGame|SaveJournalData(Message) :self (Game|GetGameInstance)))

(fn ConstructionScript)