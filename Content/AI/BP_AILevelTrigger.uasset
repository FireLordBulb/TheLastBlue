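; BP_AILevelTrigger is a trigger actor that advances the spirit AI to a new stage.
; On its first overlap, it calls SetSpiritStage on its SpiritPawn reference if ShouldChangeLevel is set, without filtering the overlapping actor.
; End overlap only casts to BP_SpiritPawn.
; Smoke toggling, Niagara fire resizing and SpiritManager stage-setting with debug prints remain as disconnected, unused logic.
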(event EventBeginPlay
  (|CallParentFunction))

(event Collision|EventActorBeginOverlap
  (params (OtherActor :type Actor%20Object%20Reference))
  (|CallParentFunction OtherActor)
  (Utilities|FlowControl|DoOnce false
    (:Completed
      (if (Variables|Default|GetshouldChangeLevel)
        (Default|SetSpiritStage (Variables|Default|GetSpiritPawn) (Variables|Default|GetNew%20Stage))))))

(event EventTick
  (params (DeltaSeconds :type Float%20%28single-precision%29)))

(event Collision|EventActorEndOverlap
  (params (OtherActor :type Actor%20Object%20Reference))
  (Utilities|Casting|CastToBP_SpiritPawn OtherActor))

(fn ConstructionScript
  (|CallParentFunction))