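; BP_SpiritPawn is the AI-controlled spirit pawn that stays near the player, with a dialogue widget and a Niagara fire effect.
; Once the player has been within close range, Tick teleports it onto them whenever they exceed the maximum distance.
; BeginPlay restores saved transform and AI state, which GetSpiritData exposes through the SpiritAIController.
; ChangeFireSize adjusts the fire's size and colour, then its spawn rate after a delay.
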(event Custom|ChangeFireSize
  (params (FireSize :type Float%20%28double-precision%29) (spawnRate :type Float%20%28double-precision%29))
  (bind _spiritfire (Variables|Default|GetSpiritFire))
  (Niagara|SetNiagaraVariable(Float) _spiritfire "User.FireSize" FireSize)
  (Development|PrintString "changed")
  (Niagara|SetNiagaraVariable(LinearColor) _spiritfire "User.ColourMaximum" (Utilities|Struct|MakeLinearColor 255.0 0.0 0.0 1.0))
  (Utilities|FlowControl|Delay 0.2)
  (Niagara|SetNiagaraVariable(Float) (Variables|Default|GetSpiritFire) "User.spawnRate" spawnRate))

(event EventBeginPlay
  (Utilities|FlowControl|Sequence
    (:then_0
      (Class|GlyphProvider|OverrideRenderTarget (Variables|Default|GetSpiritDialogGlyphProvider) "/Game/Spirit/RT_SpiritDialog.RT_SpiritDialog")
      (bind _asspirit_dialogue_widget (Utilities|Casting|CastToSpiritDialogueWidget (UserInterface|GetWidget (Variables|Default|GetWidget)))
        (:then
          (Variables|Default|SetDialogueElement _asspirit_dialogue_widget))
        (:CastFailed
          _))
      ;[1 1 1] Set Spirit Save Data
      (bind _returnvalue (SaveGame|DoesSaveGameExist (Variables|Default|GetSaveSlot)))
      (if _returnvalue
        (bind _savegame (Class|BPISaveGame|GetGameData(Message) (Game|GetGameInstance)))
        (Utilities|IsValid _savegame
          (:Is%20Valid
            (CallFunction|SetSpiritData (Variables|/Game/SaveGame/BP_SaveGame.BP_SaveGame_C|GetSpiritSaveData _savegame))))))
    (:then_1
      (Variables|Default|SetPlayerPawn (Game|Player|GetPlayerPawn 0)))))

(event EventTick
  (params (DeltaSeconds :type Float%20%28single-precision%29))
  (bind _returnvalue (Transformation|GetActorLocation))
  (bind _playerpawn (Variables|Default|GetPlayerPawn))
  (bind _returnvalue_2 (Transformation|GetActorLocation _playerpawn))
  (bind _returnvalue_3 (Math|Vector|Distance(Vector) _returnvalue_2 _returnvalue))
  (if (Variables|Default|GetPlayerHasBeenClose)
    (Math|Float|CompareFloat (Variables|Default|GetMaxDistance) _returnvalue_3
      (:<
        (Transformation|SetActorLocation (Transformation|GetActorLocation (Variables|Default|GetPlayerPawn)) false true)))
    (else
      (Math|Float|CompareFloat (Variables|Default|GetCloseDistance) _returnvalue_3
        (:>
          (Variables|Default|SetPlayerHasBeenClose true))))))

(fn ConstructionScript)

(fn GetSpiritData
  (bind _asspirit_aicontroller (Utilities|Casting|CastToSpiritAIController (Pawn|GetController)))
  (return (Utilities|Struct|MakeS_SpiritSaveData (Transformation|GetActorTransform) (Class|SpiritAIStateManager|GetCurrentState (Variables|/Script/GP3_Team09.SpiritAIController|GetSpiritStateManager _asspirit_aicontroller)))))

(fn SetSpiritData
  (params (Spirit%20Save%20Data :type S%20Spirit%20Save%20Data%20Structure))
  (bind _asspirit_aicontroller (Utilities|Casting|CastToSpiritAIController (Pawn|GetController)))
  (if (not (== (.transform Spirit%20Save%20Data) (Math|Transform|MakeTransform "0, 0, 0")))
    (Transformation|SetActorTransform (.transform Spirit%20Save%20Data))
    (Class|SpiritAIController|SetAIState _asspirit_aicontroller (Utilities|Enum|ByteToEnumESpiritState (.state Spirit%20Save%20Data)))))