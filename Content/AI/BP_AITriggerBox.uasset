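; Trigger box actor that switches the Spirit AI state the first time the player character overlaps it.
; It constructs a SpiritAIStateManager on BeginPlay, then applies its configured state to it on overlap.
; For Waypoint, it also sets the waypoint index and glyph sentence and enables a polling flag.
; Tick then switches the manager to ShowGlyph whenever it is in Wait, if glyph display is enabled.
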(event OnComponentBeginOverlap(Box)
  (params (OverlappedComponent :type Primitive%20Component%20Object%20Reference) (OtherActor :type Actor%20Object%20Reference) (OtherComp :type Primitive%20Component%20Object%20Reference) (OtherBodyIndex :type Integer) (bFromSweep :type Boolean) (SweepResult :type Hit%20Result%20Structure%20%28by%20ref%29))
  (bind _new_state (Variables|Default|GetNew%20State))
  (Utilities|Casting|CastToBP_PlayerCharacter OtherActor)
  (Utilities|FlowControl|DoOnce false
    (:Completed
      (Utilities|FlowControl|Sequence
        (:then_0
          (Class|SpiritAIStateManager|ChangeState (Variables|Default|GetSpirit%20Manager) _new_state)
          (Development|PrintString (Utilities|String|EnumtoString _new_state))
          (if (Utilities|Enum|Equal(Enum) (Variables|Default|GetNew%20State) "Waypoint")
            (Class|SpiritAIStateManager|SetWaypointIndex (Variables|Default|GetSpirit%20Manager) (Variables|Default|GetWapointNumber))
            (Class|SpiritAIStateManager|ChangeGlyph (Variables|Default|GetSpirit%20Manager) (Variables|Default|GetHeldSetence))
            (Variables|Default|SetactivateTick true)))))))

(event EventTick
  (params (DeltaSeconds :type Float%20%28single-precision%29))
  (Utilities|FlowControl|Sequence
    (:then_0
      (if (Variables|Default|GetactivateTick)
        (if (Variables|Default|GetshouldShowGlyph)
          (if (Utilities|Enum|Equal(Enum) (Class|SpiritAIStateManager|GetCurrentState (Variables|Default|GetSpirit%20Manager)) "Wait")
            (Class|SpiritAIStateManager|ChangeState (Variables|Default|GetSpirit%20Manager) "ShowGlyph")
            (Class|Actor|RemoveTickPrerequisiteActor)
            (Development|PrintString "Hello")))))))

(event EventBeginPlay
  (bind _returnvalue (Game|ConstructObjectfromClass "/Script/GP3_Team09.SpiritAIStateManager"))
  (Variables|Default|SetSpirit%20Manager _returnvalue))

(fn ConstructionScript)