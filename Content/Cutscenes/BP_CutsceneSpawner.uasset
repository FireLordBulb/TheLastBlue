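; Trigger actor that plays the outro cutscene when the player character enters its box, then returns the game to the main menu.
; The first valid overlap, gated by DoOnce, calls DisableInput on this actor with the player's controller, adds WBP_Cutscene to the viewport and opens the outro source on a media player.
; The media player's OnEndReached event fires CutsceneEnded, which opens the MainMenu level.
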(event OnComponentBeginOverlap(Box)
  (params (OverlappedComponent :type Primitive%20Component%20Object%20Reference) (OtherActor :type Actor%20Object%20Reference) (OtherComp :type Primitive%20Component%20Object%20Reference) (OtherBodyIndex :type Integer) (bFromSweep :type Boolean) (SweepResult :type Hit%20Result%20Structure%20%28by%20ref%29))
  (bind _mediaplayerref (Variables|Default|GetMediaPlayerRef))
  (bind _asbp_player_character (Utilities|Casting|CastToBP_PlayerCharacter OtherActor))
  (Utilities|FlowControl|DoOnce false
    (:Completed
      (Input|DisableInput (Pawn|GetLocalViewingPlayerController _asbp_player_character))
      (bind _returnvalue (UserInterface|CreateWidget "/Game/Cutscenes/WBP_Cutscene.WBP_Cutscene_C"))
      (Variables|Default|SetWBPCutscene _returnvalue)
      (UserInterface|Viewport|AddtoViewport (Variables|Default|GetWBPCutscene) 0)
      (Media|MediaPlayer|OpenSource _mediaplayerref "/Game/Art/Videos/OutroCutScene.OutroCutScene")
      (Media|MediaPlayer|BindEventtoOnEndReached _mediaplayerref (delegate Custom|CutsceneEnded)))))

(event Custom|CutsceneEnded
  (Game|OpenLevel(byObjectReference) "/Game/Maps/MainMenu.MainMenu"))

(event EventBeginPlay)

(event Collision|EventActorBeginOverlap
  (params (OtherActor :type Actor%20Object%20Reference)))

(event EventTick
  (params (DeltaSeconds :type Float%20%28single-precision%29)))

(fn ConstructionScript)