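; BP_DoorOpener is a prototype actor that drives a two-door sequence for what appears to be an intro area.
; Power on opens the first door and disables the energy sources of "Intro"-tagged BP_EnergySocket actors cached at BeginPlay; power off reverses both.
; Overlapping its hitbox closes the first door, then opens the second after a short delay.
; Helper functions check each door's open state before toggling it.
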(event OnComponentBeginOverlap(Hitbox)
  (params (OverlappedComponent :type Primitive%20Component%20Object%20Reference) (OtherActor :type Actor%20Object%20Reference) (OtherComp :type Primitive%20Component%20Object%20Reference) (OtherBodyIndex :type Integer) (bFromSweep :type Boolean) (SweepResult :type Hit%20Result%20Structure%20%28by%20ref%29))
  (CallFunction|CloseCurrentDoor (Variables|Default|GetFirstDoor))
  (Utilities|FlowControl|Delay 2.0)
  (CallFunction|OpenCurrentDoor (Variables|Default|GetSecondDoor)))

(event EventBeginPlay
  (bind _outactors (Actor|GetAllActorsOfClasswithTag "/Game/PuzzleObjects/BP_EnergySocket.BP_EnergySocket_C" "Intro"))
  (Variables|Default|SetSpheres%20to%20Disable%20Array _outactors))

(event EventOnPoweron
  (CallFunction|OpenCurrentDoor (Variables|Default|GetFirstDoor))
  (for _array_element (Variables|Default|GetSpheres%20to%20Disable%20Array)
    (Class|Interaction|SetEnabled (Variables|/Game/PuzzleObjects/BP_EnergySocket.BP_EnergySocket_C|GetEnergySource _array_element) false)))

(event EventOnPowerOff
  (CallFunction|CloseCurrentDoor (Variables|Default|GetFirstDoor))
  (for _array_element (Variables|Default|GetSpheres%20to%20Disable%20Array)
    (Class|Interaction|SetEnabled (Variables|/Game/PuzzleObjects/BP_EnergySocket.BP_EnergySocket_C|GetEnergySource _array_element) true)))

(fn ConstructionScript)

(fn OpenCurrentDoor
  (params (Door :type BP%20Door%20Object%20Reference))
  (if (not (Variables|/Script/GP3_Team09.PuzzleDoor|GetIsOpen Door))
    (Default|OpenDoor Door)))

(fn CloseCurrentDoor
  (params (Door :type BP%20Door%20Object%20Reference))
  (if (Variables|/Script/GP3_Team09.PuzzleDoor|GetIsOpen Door)
    (Default|CloseDoor Door)))

(fn GetGlyphProvider
  (return 0))