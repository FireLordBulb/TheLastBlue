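; BP_Tutorials is a trigger actor that shows a one-time tutorial prompt when a player-tagged actor overlaps its TutBox.
; On BeginPlay it creates a WBP_TutorialPrompts widget and adds it to the viewport.
; The first valid overlap passes TutorialText to the widget, reveals it and starts a ShowTime timer.
; When the timer fires, CloseTutorial plays the scale animation in reverse, then removes the widget after a short delay.
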(event OnComponentBeginOverlap(TutBox)
  (params (OverlappedComponent :type Primitive%20Component%20Object%20Reference) (OtherActor :type Actor%20Object%20Reference) (OtherComp :type Primitive%20Component%20Object%20Reference) (OtherBodyIndex :type Integer) (bFromSweep :type Boolean) (SweepResult :type Hit%20Result%20Structure%20%28by%20ref%29))
  ;[1 1 1] On Collision Display Text
  (if (not (Variables|Default|Getshown))
    (if (Actor|ActorHasTag OtherActor "player")
      (Variables|/Game/Prototypes/WBP_TutorialPrompts.WBP_TutorialPrompts_C|SettutorialText (Variables|Default|GettutorialWidget) (Variables|Default|GettutorialText))
      (Variables|/Script/UMG.Widget|SetVisibility (Variables|Default|GettutorialWidget) "SelfHitTestInvisible")
      (Utilities|Time|SetTimerbyEvent (delegate Custom|CloseTutorial) (Variables|Default|GetshowTime))
      (Variables|Default|Setshown true))))

(event Custom|CloseTutorial
  (bind _tutorialwidget (Variables|Default|GettutorialWidget))
  ;[1 1 1] On Collision Display Text
  (UserInterface|Animation|PlayAnimation _tutorialwidget (Variables|/Game/Prototypes/WBP_TutorialPrompts.WBP_TutorialPrompts_C|GetScaleAnimation _tutorialwidget) 0.0 1 "Reverse" 1.0 false)
  (Utilities|FlowControl|Delay 2.0)
  (Widget|RemovefromParent (Variables|Default|GettutorialWidget)))

(event EventBeginPlay
  ;[1 1 1] Widget Creation
  (Utilities|IsValid (Variables|Default|GettutorialWidget)
    (:Is%20Not%20Valid
      (bind _returnvalue (UserInterface|CreateWidget "/Game/Prototypes/WBP_TutorialPrompts.WBP_TutorialPrompts_C" (Game|GetPlayerController 0)))
      (bind _output_get (Variables|Default|SettutorialWidget _returnvalue))
      (UserInterface|Viewport|AddtoViewport _output_get 0)
      (Variables|Default|Setshown false))))

(fn ConstructionScript)