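; BP_BallSmall is a prototype ball that changes size each time its Interaction component fires.
; Interactions step a wrapping index through normal, double, normal and half scales built at BeginPlay, setting ObjectState from a parallel array.
; A Timeline lerps the relative scale, ignoring further interactions until it finishes.
; An older bitmask-branching version remains in functions marked redundant, which the event graph never calls.
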(event Custom|SizeChangeInteraction
  (if (not (Variables|Default|GetIsScaling))
    (Variables|Default|SetStateIndex (Math|Integer|%(Integer) (+ (Variables|Default|GetStateIndex) 1) (Utilities|Array|Length (Variables|Default|GetTargetScales))))
    (Variables|Default|SetTargetScale (Utilities|Array|Get(acopy) (Variables|Default|GetTargetScales) (Variables|Default|GetStateIndex)))
    (Variables|Default|SetObjectState (Utilities|Array|Get(acopy) (Variables|Default|GetObjectStates) (Variables|Default|GetStateIndex)))
    (Variables|Default|SetIsScaling true)
    (bind _set_scale_alpha (Timeline|Timeline_0 PlayFromStart)
      (:Update
        (Transformation|SetActorRelativeScale3D (Math|Vector|Lerp(Vector) (Variables|Default|GetCurrentScale) (Variables|Default|GetTargetScale) _set_scale_alpha)))
      (:Finished
        (Variables|Default|SetIsScaling false)
        (Variables|Default|SetCurrentScale (Variables|Default|GetTargetScale))))))

(event EventBeginPlay
  (|CallParentFunction)
  (Variables|Default|SetObjectState 64)
  (bind _output_get (Variables|Default|SetDefaultScale (Transformation|GetActorScale3D)))
  (Variables|Default|SetCurrentScale _output_get)
  (EventDispatchers|BindEventtoInteracted (Variables|Default|GetInteraction) (delegate Custom|SizeChangeInteraction))
  (Variables|Default|SetTargetScales (Utilities|Array|MakeArray (Variables|Default|GetDefaultScale) (* (Variables|Default|GetDefaultScale) 2.0) (Variables|Default|GetDefaultScale) (/ (Variables|Default|GetDefaultScale) 2.0))))

(fn ConstructionScript
  (|CallParentFunction))

(fn EvaluateInteractionREDUNDANT
  (if (Utilities|TestBit (Variables|Default|GetObjectState) (|BitmaskLiteral))
    (CallFunction|EnlargeREDUNDANT)
    (elif (Utilities|TestBit (Variables|Default|GetObjectState) (|BitmaskLiteral 2))
      (CallFunction|ReturntoDefaultfromEnlargedREDUNTDANT)
      (elif (Utilities|TestBit (Variables|Default|GetObjectState) (|BitmaskLiteral 4))
        (CallFunction|ShrinkREDUNTDANT)
        (elif (Utilities|TestBit (Variables|Default|GetObjectState) (|BitmaskLiteral 1))
          (CallFunction|ReturntoDefaultfromShrunkREDUNTDANT))))))

(fn ShrinkREDUNTDANT
  (Variables|Default|SetTargetScale (/ (Variables|Default|GetCurrentScale) 2.0))
  (Variables|Default|SetObjectState 1))

(fn ReturntoDefaultfromShrunkREDUNTDANT
  (Variables|Default|SetTargetScale (Variables|Default|GetDefaultScale))
  (Variables|Default|SetObjectState 64))

(fn ReturntoDefaultfromEnlargedREDUNTDANT
  (Variables|Default|SetTargetScale (Variables|Default|GetDefaultScale))
  (Variables|Default|SetObjectState 4))

(fn EnlargeREDUNDANT
  (Variables|Default|SetTargetScale (* (Variables|Default|GetCurrentScale) 2.0))
  (Variables|Default|SetObjectState 2))