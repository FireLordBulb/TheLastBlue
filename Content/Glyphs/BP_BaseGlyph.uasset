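; Base interactable glyph puzzle that the player edits by cycling sub-glyph symbols to match required meanings.
; Interacting toggles editing, moving PlayerGlyphEditor and the camera onto the glyph.
; A per-tick mouse trace highlights the nearest-in-radius sub-glyph with an emissive material, and clicks cycle its symbol, updating BPGlyphProvider, whose texture feeds the display.
; Exiting validates RequiredWords, calls empty OnValid/OnInvalid hooks and confirms the glyph.
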(event Custom|Interacted%20Event
  (bind _returnvalue (Game|GetPlayerController 0))
  (bind _interaction (Variables|Default|GetInteraction))
  (bind _returnvalue_2 (Pawn|GetControlledPawn _returnvalue))
  (bind _instancespawnwidget (Variables|/Script/GP3_Team09.Interaction|GetInstanceSpawnWidget _interaction))
  (bind _returnvalue_3 (Actor|GetComponentbyClass _returnvalue_2 "/Script/GP3_Team09.PlayerGlyphEditor"))
  (bind _returnvalue_4 (Actor|GetComponentbyClass _returnvalue_2 "/Game/PlayerCharacter/BP_PlayerCamera.BP_PlayerCamera_C"))
  (bind _returnvalue_5 (UserInterface|GetWidget _instancespawnwidget))
  ;[0.8553 0.2654 1] Glyph Editing Start/Stop
  (bind _output_get (Variables|Default|SetIsBeingUsed (not (Variables|Default|GetIsBeingUsed))))
  (Variables|/Script/Engine.PlayerController|SetbShowMouseCursor _returnvalue _output_get)
  (Utilities|IsValid _returnvalue_3
    (:Is%20Valid
      (Utilities|IsValid _returnvalue_4
        (:Is%20Valid
          (bind _output_get_2 (Variables|/Script/GP3_Team09.PlayerGlyphEditor|SetbGlyphEditingIsActive _returnvalue_3 _output_get))
          (if _output_get_2
            (Variables|/Script/GP3_Team09.PlayerGlyphEditor|SetGlyph _returnvalue_3 self)
            (Default|SetTargetTransform _returnvalue_4 (Variables|Default|GetStatic%20Camera%20Transform))
            (Utilities|IsValid _returnvalue_5
              (:Is%20Valid
                (Variables|/Script/UMG.Widget|SetVisibility _returnvalue_5 "Collapsed")))
            (else
              (Variables|/Script/GP3_Team09.PlayerGlyphEditor|SetGlyph _returnvalue_3 0)
              (Default|ReturntoPlayer _returnvalue_4)
              (Utilities|IsValid _returnvalue_5
                (:Is%20Valid
                  (Variables|/Script/UMG.Widget|SetVisibility _returnvalue_5 "Visible")
                  ;[0.6151 1 0.09082] Glyph validation, both old and new
                  (bind _isvalid (CallFunction|ValidateGlyph))
                  (if _isvalid
                    (CallFunction|OnValid)
                    (else
                      (CallFunction|OnInvalid)))
                  (Class|GlyphProvider|ConfirmGlyph (Variables|Default|GetBP_GlyphProvider))
                  (Utilities|UnselectSelectedSubGlyph))))))
        (:Is%20Not%20Valid
          (Development|PrintString "Missing Component on PlayerCharacter!" :!label _label))))
    (:Is%20Not%20Valid
      (goto _label))))

(event Custom|Pointing%20Event
  (params (Value :type Interaction%20Object%20Reference))
  (Development|PrintString "Pointed"))

(event EventOnReceiveClickInput
  (bind _selectedsubglyph (Variables|Default|GetSelectedSubGlyph))
  ;[0.3431 1 0.7003] Glyph Editing On Input
  (Utilities|IsValid _selectedsubglyph
    (:Is%20Valid
      (CallFunction|CycleSubGlyphMaterial _selectedsubglyph true))))

(event EventBeginPlay
  (bind _returnvalue (Actor|GetComponentbyClass "/Script/GP3_Team09.Interaction"))
  (Utilities|IsValid _returnvalue
    (:Is%20Valid
      (bind _output_get (Variables|Default|SetInteraction _returnvalue)))
    (:Is%20Not%20Valid
      (bind _returnvalue_2 (Game|AddComponentbyClass "/Game/PuzzleObjects/BP_Interaction.BP_Interaction_C"))
      (bind _output_get_2 (Variables|Default|SetInteraction _returnvalue_2))))
  (EventDispatchers|BindEventtoGlyphInteracted _output_get (delegate Custom|Interacted%20Event))
  (if (Variables|/Script/GP3_Team09.Interaction|GetCanPointToSpirit _output_get)
    (EventDispatchers|BindEventtoPointed (Variables|Default|GetInteraction) (delegate Custom|Pointing%20Event)))
  ;[0.3065 0.3381 1] Setup Sub Glyph Materials
  (Variables|/Script/GP3_Team09.SubGlyph|SetTempMesh (Variables|Default|GetBP_BaseSubGlyph1) (Variables|Default|GetSubGlyphMesh1))
  (Variables|/Script/GP3_Team09.SubGlyph|SetTempMesh (Variables|Default|GetBP_BaseSubGlyph2) (Variables|Default|GetSubGlyphMesh2))
  (Variables|/Script/GP3_Team09.SubGlyph|SetTempMesh (Variables|Default|GetBP_BaseSubGlyph3) (Variables|Default|GetSubGlyphMesh3))
  (for _array_element (Actor|GetComponentsByClass "/Script/GP3_Team09.SubGlyph")
    (CallFunction|UpdateSubGlyphMaterial _array_element false)))

(event EventTick
  (params (DeltaSeconds :type Float%20%28single-precision%29))
  ;[1 0.1534 0.1136] Check which SubGlyph is hovered
  (if (Variables|Default|GetIsBeingUsed)
    (CallFunction|UpdateSelectedSubGlyph)))

(fn ConstructionScript
  (Variables|Glyph|SetCurrentSentence (Variables|Glyph|GetDefaultSentence))
  (CallFunction|ResetDisplay))

(fn UpdateSubGlyphMaterial
  (params (SubGlyph :type Sub%20Glyph%20Object%20Reference) (IsEmissive :type Boolean))
  (bind _returnvalue (Rendering|Material|CreateDynamicMaterialInstance (select (and IsEmissive (Variables|/Script/GP3_Team09.SubGlyph|GetbIsEditable SubGlyph)) "/Game/Glyphs/Materials/M_SubGlyphEmissive.M_SubGlyphEmissive" "/Game/Glyphs/Materials/M_SubGlyph.M_SubGlyph") "None" "None" :!class /Script/Engine.KismetMaterialLibrary))
  (Rendering|Material|SetTextureParameterValue _returnvalue "GlyphTexture" (.texture (Utilities|GetCurrentSymbol SubGlyph)))
  (Rendering|Material|SetMaterial (Variables|/Script/GP3_Team09.SubGlyph|GetTempMesh SubGlyph) 0 _returnvalue))

(fn SetSubGlyphMaterial
  (params (SubGlyph :type Sub%20Glyph%20Object%20Reference) (SymbolIndex :type Integer) (IsEmissive :type Boolean))
  (bind _currentsymbol (Utilities|GetCurrentSymbol SubGlyph))
  (if (Variables|/Script/GP3_Team09.SubGlyph|GetbIsEditable SubGlyph)
    (Variables|/Script/GP3_Team09.SubGlyph|SetCurrentSymbolIndex SubGlyph SymbolIndex)
    (CallFunction|UpdateSubGlyphMaterial SubGlyph IsEmissive)
    (Class|GlyphProvider|SetMinorGlyph (Variables|Default|GetBP_GlyphProvider) 0 (.position _currentsymbol) (.word _currentsymbol))
    (Development|PrintString (.word _currentsymbol))))

(fn CycleSubGlyphMaterial
  (params (SubGlyph :type Sub%20Glyph%20Object%20Reference) (IsEmissive :type Boolean))
  (CallFunction|SetSubGlyphMaterial SubGlyph (Math|Integer|%(Integer) (+ (Variables|/Script/GP3_Team09.SubGlyph|GetCurrentSymbolIndex SubGlyph) 1) (Utilities|Array|Length (Variables|/Script/GP3_Team09.SubGlyph|GetSymbols SubGlyph))) IsEmissive))

(fn UpdateSelectedSubGlyph
  (bind _returnvalue (Game|GetPlayerController 0))
  (bind (_worldlocation _worlddirection) (Game|Player|ConvertMouseLocationToWorldSpace _returnvalue))
  ;[1 0.7901 0.1603] Line Trace the mouse position
  (bind _outhit (Collision|LineTraceByChannel _worldlocation (+ _worldlocation (* _worlddirection 1e+03)) "TraceTypeQuery1" false 0 "None" false))
  (if (.bblockinghit _outhit)
    ;[0.2914 0.7129 1] Check if any glyph is close enough that it counts as a mouse hover
    (for _array_element (Actor|GetComponentsByClass "/Script/GP3_Team09.SubGlyph")
      (Math|Float|CompareFloat (Variables|Default|GetSubGlyphClickRadius) (Math|Vector|Distance(Vector) (Transformation|GetWorldLocation _array_element) (.location _outhit))
        (:>
          (if (!= _array_element (Variables|Default|GetSelectedSubGlyph))
            (bind _output_get (Variables|Default|SetSelectedSubGlyph _array_element))
            (CallFunction|UpdateSubGlyphMaterial _output_get true)
            (return)
            (else
              (return)))))))
  (Utilities|UnselectSelectedSubGlyph))

(fn ValidateGlyph
  (bind _array_element (Utilities|Array|ForEachLoopwithBreak (Actor|GetComponentsByClass "/Script/GP3_Team09.SubGlyph"))
    (:LoopBody
      (Utilities|Array|Add (LocalVariables|GetCurrentWords) (.meaning (Utilities|GetCurrentSymbol _array_element))))
    (:Completed
      (bind _array_element_2 (Utilities|Array|ForEachLoopwithBreak (Variables|Default|GetRequiredWords) :!label _label)
        (:LoopBody
          (if (not (Utilities|Array|ContainsItem (LocalVariables|GetCurrentWords) _array_element_2))
            (LocalVariables|SetHasAllWords false)
            (goto _label Break)))
        (:Completed
          (return (LocalVariables|GetHasAllWords)))))))

(fn OnValid)

(fn OnInvalid)

(fn ResetDisplay
  (bind _bp_glyphprovider (Variables|Default|GetBP_GlyphProvider))
  (bind _returnvalue (Class|GlyphProvider|GetTextureRef (Variables|Default|GetBP_GlyphProvider)))
  (bind _returnvalue_2 (Rendering|Material|CreateDynamicMaterialInstance (Variables|Default|GetDisplay) :!class /Script/Engine.DecalComponent))
  (Rendering|Material|SetTextureParameterValue _returnvalue_2 "GlyphRT" _returnvalue)
  (bind _returnvalue_3 (Class|GlyphProvider|SetSentence _bp_glyphprovider (Variables|Glyph|GetCurrentSentence)))
  (if _returnvalue_3
    (Class|GlyphProvider|CreateInitialGlyph _bp_glyphprovider)
    (else
      (Development|PrintString "failed to assign a sentence to a glyph provider"))))