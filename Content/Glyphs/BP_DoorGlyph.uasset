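; BP_DoorGlyph is a glyph puzzle Blueprint that opens or closes a referenced door based on a required word sequence.
; On BeginPlay it runs the parent logic, then sets the required words to Door, Is, Open.
; It implements OnValid to open the door and OnInvalid to close it, each only if the Door reference is valid.
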(event EventBeginPlay
  (|CallParentFunction)
  (Variables|Default|SetRequiredWords (Utilities|Array|MakeArray "Door" "Is" "Open")))

(fn ConstructionScript
  (|CallParentFunction))

(fn OnValid
  (bind _door (Variables|Default|GetDoor))
  (Utilities|IsValid _door
    (:Is%20Valid
      (Default|OpenDoor _door))))

(fn OnInvalid
  (bind _door (Variables|Default|GetDoor))
  (Utilities|IsValid _door
    (:Is%20Valid
      (Default|CloseDoor _door))))