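; Holographic glyph display actor that unfolds a plane showing a glyph when the player overlaps it, and folds it away when they leave.
; The construction script feeds the glyph provider's texture into a dynamic material on the plane and creates the initial glyph.
; A timeline, played or reversed on overlap, scales the plane's X and Y from zero.
; While enabled, Tick rotates the whole actor toward the player using a world-up look-at.
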(event EventBeginPlay
  (bind _plane (Variables|Default|GetPlane))
  (|CallParentFunction)
  (Variables|References|SetPlayerRef (Game|Player|GetPlayerPawn 0))
  (Components|Timeline|SetPlayRate (Variables|Default|GetActivationTimeLine) (Variables|Animation|GetactivationAnimSpeed))
  (Variables|Animation|SetdefaultPlaneScale (Variables|/Script/Engine.SceneComponent|GetRelativeScale3D _plane))
  (Transformation|SetRelativeScale3D _plane "0, 0, 0"))

(event Collision|EventActorBeginOverlap
  (params (OtherActor :type Actor%20Object%20Reference))
  (|CallParentFunction 0)
  (if (== OtherActor (Variables|References|GetPlayerRef))
    (Variables|Animation|SetbDisplayEnabled true)
    (bind _activationanim (Timeline|ActivationTimeLine Play)
      (:Update
        (Transformation|SetRelativeScale3D (Variables|Default|GetPlane) (* (Math|Vector|MakeVector (.X (Class|KismetMathLibrary|BreakVector3f _activationanim)) (.Y (Class|KismetMathLibrary|BreakVector3f _activationanim)) 1.0) (Variables|Animation|GetdefaultPlaneScale)))))))

(event EventTick
  (params (DeltaSeconds :type Float%20%28single-precision%29))
  (|CallParentFunction DeltaSeconds)
  (if (Variables|Animation|GetbDisplayEnabled)
    (CallFunction|FacePlayer)))

(event Collision|EventActorEndOverlap
  (params (OtherActor :type Actor%20Object%20Reference))
  (|CallParentFunction OtherActor)
  (if (== OtherActor (Variables|References|GetPlayerRef))
    (Variables|Animation|SetbDisplayEnabled false)
    (bind _activationanim (Timeline|ActivationTimeLine Reverse)
      (:Update
        (Transformation|SetRelativeScale3D (Variables|Default|GetPlane) (* (Math|Vector|MakeVector (.X (Class|KismetMathLibrary|BreakVector3f _activationanim)) (.Y (Class|KismetMathLibrary|BreakVector3f _activationanim)) 1.0) (Variables|Animation|GetdefaultPlaneScale)))))))

(fn ConstructionScript
  (bind _plane (Variables|Default|GetPlane))
  (bind _returnvalue (Class|GlyphProvider|GetTextureRef (Variables|Default|GetBP_GlyphProvider)))
  (bind _returnvalue_2 (Rendering|Material|CreateDynamicMaterialInstance _plane 0 (Rendering|Material|GetMaterial _plane 0) "HoloMatInstance" :!class /Script/Engine.PrimitiveComponent))
  (Rendering|Material|SetTextureParameterValue _returnvalue_2 "GlyphRT" _returnvalue)
  (Class|GlyphProvider|CreateInitialGlyph (Variables|Default|GetBP_GlyphProvider))
  (|CallParentFunction))

(fn FacePlayer
  (Transformation|SetActorTransform (Class|KismetAnimationLibrary|Lookat (Transformation|GetActorTransform) (Transformation|GetActorLocation (Variables|References|GetPlayerRef)) "-1.000000,0.000000,0.000000" true "0.000000,0.000000,1.000000" 0.0)))

(fn Reset
  (|CallParentFunction))