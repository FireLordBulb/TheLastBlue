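; BP_GlyphCombiner links groups of glyph sentence displays, called murals, to the player's journal.
; On BeginPlay it builds a sentence collection per mural and caches the journal toggler from the player character.
; When given a sentence display, it adds missing words from the whole matching mural, enables that mural's journal entry by index and notifies the toggler on success.
; Displays outside any mural add only their own words.
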(event EventBeginPlay
  (CallFunction|BeginSetup))

(event Collision|EventActorBeginOverlap
  (params (OtherActor :type Actor%20Object%20Reference)))

(event EventTick
  (params (DeltaSeconds :type Float%20%28single-precision%29)))

(fn ConstructionScript)

(fn GetSentences
  (params (Displays :type Array%20of%20A%20Interactive%20Glyph%20Display%20Object%20References))
  (for _array_element Displays
    (Utilities|Array|Add (LocalVariables|GetTempSentences) (Variables|/Game/Glyphs/A_GlyphDisplay.A_GlyphDisplay_C|GetDefaultSentence _array_element)))
  (return (LocalVariables|GetTempSentences)))

(fn GetSentencesCollection
  (for _array_element (Variables|Default|GetMurals)
    (bind _sentences (CallFunction|GetSentences (Utilities|Struct|BreakFU_GlyphCombiner _array_element)))
    (Utilities|Array|Add (Variables|Default|GetMuralsSentences) (Utilities|Struct|MakeS_SentenceCollection _sentences))))

(fn BeginSetup
  (CallFunction|GetSentencesCollection)
  (bind _returnvalue (Actor|GetActorOfClass "/Game/PlayerCharacter/BP_PlayerCharacter.BP_PlayerCharacter_C"))
  (Variables|Default|SetToggler (Variables|/Game/PlayerCharacter/BP_PlayerCharacter.BP_PlayerCharacter_C|GetBP_JournalToggler _returnvalue)))

(fn GiveSentencesJournal
  (params (Sentence :type A%20Interactive%20Glyph%20Display%20Object%20Reference))
  (for (_array_element _array_index) (Variables|Default|GetMurals)
    (if (Utilities|Array|ContainsItem (Utilities|Struct|BreakFU_GlyphCombiner _array_element) Sentence)
      (for _array_element_2 (Utilities|Struct|BreakFU_GlyphCombiner _array_element)
        (Class|PlayerWordCollection|AddMissingWordsfromSentence (Variables|/Game/Prototypes/WBP_JournalPrototype.WBP_JournalPrototype_C|GetWordCollection (Variables|Default|GetJournal)) (Variables|/Game/Glyphs/A_GlyphDisplay.A_GlyphDisplay_C|GetDefaultSentence _array_element_2)) ; some visual feedback here would be nice
      )
      (bind _added (Default|EnableSentence (Variables|Default|GetJournal) _array_index))
      (if _added
        (Default|AddSentence (Variables|Default|GetToggler)))
      (return)))
  (Class|PlayerWordCollection|AddMissingWordsfromSentence (Variables|/Game/Prototypes/WBP_JournalPrototype.WBP_JournalPrototype_C|GetWordCollection (Variables|Default|GetJournal)) (Variables|/Game/Glyphs/A_GlyphDisplay.A_GlyphDisplay_C|GetDefaultSentence Sentence)) ; some visual feedback here would be nice
  (return))