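; BP_Brush_PickUp is a brush pickup actor that gates access to a glyph display and glyph tutorial.
; BeginPlay binds its Interaction events and disables the display's ExamineInteraction and the tutorial's collision.
; Interacting hides the brush and re-enables both, while the Pointing handler is empty.
; Tick spins the static mesh by a fixed yaw step each frame, independent of delta time.
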(event Custom|PickupBrush
  (Rendering|SetActorHiddenInGame true)
  (Class|Interaction|SetEnabled (Variables|/Game/Glyphs/A_InteractiveGlyphDisplay.A_InteractiveGlyphDisplay_C|GetExamineInteraction (Variables|Default|GetGlyphDisplay)) true)
  (Collision|SetActorEnableCollision (Variables|Default|GetGlyphTutorial) true))

(event Custom|Pointing
  (params (Value :type Interaction%20Object%20Reference)))

(event EventBeginPlay
  (bind _interaction (Variables|Default|GetInteraction))
  (EventDispatchers|BindEventtoInteracted _interaction (delegate Custom|PickupBrush))
  (EventDispatchers|BindEventtoPointed _interaction (delegate Custom|Pointing))
  (Class|Interaction|SetEnabled (Variables|/Game/Glyphs/A_InteractiveGlyphDisplay.A_InteractiveGlyphDisplay_C|GetExamineInteraction (Variables|Default|GetGlyphDisplay)) false)
  (Collision|SetActorEnableCollision (Variables|Default|GetGlyphTutorial) false))

(event EventTick
  (params (DeltaSeconds :type Float%20%28single-precision%29))
  (bind _staticmeshcomponent (Variables|Debug|GetStaticMeshComponent))
  (bind _relativerotation (Variables|/Script/Engine.SceneComponent|GetRelativeRotation _staticmeshcomponent))
  (Transformation|SetRelativeRotation (Variables|Debug|GetStaticMeshComponent) (Math|Rotator|MakeRotator (.roll _relativerotation) (.pitch _relativerotation) (+ (.yaw _relativerotation) 1.0)) false false))

(fn ConstructionScript)